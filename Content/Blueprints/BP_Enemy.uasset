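; BP_Enemy is a chasing enemy that ends the game when it hits the player.
; It re-issues AI MoveTo toward the player character on BeginPlay and every Tick, and expires after a fixed lifespan.
; A hit on BP_Character shows the BP_GameOver widget and mouse cursor, pauses the game and destroys the player character.
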(event `self.ReceiveBeginPlay`
  (`self.SetLifeSpan` 20.0)
  (`|AIMoveTo` self (0.0 0.0 0.0) (`GameplayStatics.GetPlayerCharacter` 0) :!label _label))

(event `self.ReceiveTick`
  (params (DeltaSeconds :type "Float (single-precision)"))
  (goto _label))

(event `self.ReceiveHit`
  (params (MyComp :type "PrimitiveComponent Object Reference") (Other :type "Actor Object Reference") (OtherComp :type "PrimitiveComponent Object Reference") (bSelfMoved :type Boolean) (HitLocation :type "Vector Structure") (HitNormal :type "Vector Structure") (NormalImpulse :type "Vector Structure") (Hit :type "HitResult Structure (by ref)"))
  (cast `/Game/Blueprints/BP_Character` Other)
  (bind _returnvalue (`|CreateWidget` "/Game/Blueprints/BP_GameOver.BP_GameOver_C"))
  (`UserWidget.AddToViewport` _returnvalue 0)
  (set `PlayerController.bShowMouseCursor` true (`GameplayStatics.GetPlayerController` 0))
  (`GameplayStatics.SetGamePaused` true)
  (`self.K2_DestroyActor` (`GameplayStatics.GetPlayerCharacter` 0)))

(fn `UserConstructionScript`)