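; BP_EnemySpawner is a spawner actor that creates escalating waves of BP_Enemy at its own transform.
; On BeginPlay it binds SpawnEnemy to the RespawnEnemy event on BP_GameMode, so the game mode triggers each wave.
; Each wave always spawns regardless of collision, then raises the increment by one and adds it to the next wave's count, so wave size grows at an accelerating rate.
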(event `self.ReceiveBeginPlay`
  (bind _asbp_game_mode (cast `/Game/Maps/BP_GameMode` (`GameplayStatics.GetGameMode`)))
  (add `/Game/Maps/BP_GameMode.RespawnEnemy` _asbp_game_mode (delegate `SpawnEnemy`)))

(event `SpawnEnemy`
  (for _ (range (`self.EnemySpawned`))
    (`|SpawnActorFromClass` "/Game/Blueprints/BP_Enemy.BP_Enemy_C" (`self.GetTransform`) "AlwaysSpawn" "OverrideRootScale" null null))
  (`/Engine/EditorBlueprintResources/StandardMacros.IncrementInt` (`self.EnemyIncrement`)
    (:`  `
      (set `self.EnemySpawned` (+ (`self.EnemySpawned`) (`self.EnemyIncrement`))))))

(fn `UserConstructionScript`)